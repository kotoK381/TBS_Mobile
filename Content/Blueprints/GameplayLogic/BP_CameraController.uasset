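; Player controller for gameplay that sets up the HUD, handles grid cell clicks and pans the camera by swiping.
; BeginPlay creates the WB_Gameplay widget and shows the cursor.
; Left click traces from the cursor against WorldDynamic objects and calls Click on a hit BP_Grid.
; Touch opens a Tick gate that, past a swipe threshold, moves BP_Camera each frame at fixed height, proportional to the offset from the touch start.
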(event `self.ReceiveBeginPlay`
  ;[1 1 1] Создание виджета и включение курсора
  (`/Engine/EditorBlueprintResources/StandardMacros.IsValid` (`self.WB_Gameplay`)
    (:`Is Not Valid`
      (bind _returnvalue (`|CreateWidget` "/Game/UI/Gameplay/WB_Gameplay.WB_Gameplay_C" (`GameplayStatics.GetPlayerController` 0)))
      (bind _output_get (set `self.WB_Gameplay` _returnvalue))
      (`UserWidget.AddToViewport` _output_get 0)
      (set `self.bShowMouseCursor` true))))

(event `Key|LeftMouseButton`
  (params (Key :type "Key Structure"))
  (bind (_worldlocation _worlddirection) (`self.DeprojectMousePositionToWorld` (`GameplayStatics.GetPlayerController` 0)))
  ;[1 1 1] Клики по ячейкам
  (:`Pressed`
    (bind (_outhit _returnvalue) (`KismetSystemLibrary.LineTraceSingleForObjects` _worldlocation (+ _worldlocation (* _worlddirection 2000.0)) (`|MakeArray` "ObjectTypeQuery2" :!type "EObjectTypeQuery Enum") false (`|MakeArray` self :!type "Actor Object Reference") "ForOneFrame" true (struct :`R` 1.0 :`A` 1.0) (struct :`G` 1.0 :`A` 1.0) 1.0))
    (if _returnvalue
      (bind _asbp_grid (cast `/Game/Blueprints/GridLogic/BP_Grid` (`.HitActor` (`GameplayStatics.BreakHitResult` _outhit))))
      (`/Game/Blueprints/GridLogic/BP_Grid.Click` _asbp_grid))))

(event `self.ReceiveTick`
  (params (DeltaSeconds :type "Float (single-precision)"))
  (bind (_locationx _locationy) (`self.GetInputTouchState` (`GameplayStatics.GetPlayerController` 0) "Touch1"))
  (bind _returnvalue (`KismetMathLibrary.MakeVector2D` _locationx _locationy))
  (bind (_returnvalue_x _returnvalue_y) (`KismetMathLibrary.BreakVector2D` (/ (- (`self.Touch_Start_2d_vector`) (`self.Touch_End_2d_vector`)) 300.0)))
  (`/Engine/EditorBlueprintResources/StandardMacros.Gate` true :!label _label
    (:`Exit`
      (if (>= (`KismetMathLibrary.VSize2D` (- _returnvalue (stale `InputTouch` _output_get))) (`self.SwipeTreshold`))
        (set `self.Touch_End_2d_vector` _returnvalue)
        (bind _asbp_camera (cast `/Game/Blueprints/GameplayLogic/BP_Camera` (`self.K2_GetPawn`)))
        (bind (_returnvalue_x_2 _returnvalue_y_2) (`KismetMathLibrary.BreakVector` (`self.K2_GetActorLocation` _asbp_camera)))
        (`self.K2_SetActorLocation` _asbp_camera (`KismetMathLibrary.MakeVector` (+ _returnvalue_x_2 (* _returnvalue_y -1.0)) (+ _returnvalue_y_2 _returnvalue_x) 112.000687) false false)))))

(event `InputTouch`
  (params (Location :type "Vector Structure") (FingerIndex :type "ETouchIndex Enum"))
  (bind (_locationx _locationy) (`self.GetInputTouchState` (`GameplayStatics.GetPlayerController` 0) "Touch1"))
  (:`Pressed`
    (bind _output_get (set `self.Touch_Start_2d_vector` (`KismetMathLibrary.MakeVector2D` _locationx _locationy)))
    (goto _label :!via `Open`))
  (:`Released`
    (goto _label :!via `Close`)))

(fn `UserConstructionScript`)