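; BP_Unit is a grid-based unit that marks tiles it can move to and travels to a selected one via AI SimpleMoveToLocation.
; Cone overlaps tint the BP_Grid underneath and set Occupied, which end overlap also leaves true.
; ShowMovingGrids matches RadiusToMove offsets from the BeginPlay location against the owning BP_Grid_Setup's grids.
; ColoringGrids then flags and tags the unoccupied matches as reachable.
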(event `self.ReceiveBeginPlay`
  (bind _output_get (set `self.MyLocation` (`self.K2_GetActorLocation`)))
  (`KismetSystemLibrary.PrintString` (`KismetStringLibrary.Conv_VectorToString` _output_get)))

(event `self.Cone.OnComponentBeginOverlap`
  (params (OverlappedComponent :type "PrimitiveComponent Object Reference") (OtherActor :type "Actor Object Reference") (OtherComp :type "PrimitiveComponent Object Reference") (OtherBodyIndex :type Integer) (bFromSweep :type Boolean) (SweepResult :type "HitResult Structure (by ref)"))
  ;[1 1 1] Подсвечивание клетки на которой стоит юнит
  (bind _asbp_grid (cast `/Game/Blueprints/GridLogic/BP_Grid` OtherActor))
  (set `/Game/Blueprints/GridLogic/BP_Grid.Occupied` true _asbp_grid)
  (`MaterialInstanceDynamic.SetVectorParameterValue` (`/Game/Blueprints/GridLogic/BP_Grid.GridMatRef` _asbp_grid) "Color" (struct :`R` 0.04474 :`B` 1.0 :`A` 1.0)))

(event `self.Cone.OnComponentEndOverlap`
  (params (OverlappedComponent :type "PrimitiveComponent Object Reference") (OtherActor :type "Actor Object Reference") (OtherComp :type "PrimitiveComponent Object Reference") (OtherBodyIndex :type Integer))
  ;[1 1 1] Подсвечивание клетки на которой стоит юнит
  (bind _asbp_grid (cast `/Game/Blueprints/GridLogic/BP_Grid` OtherActor))
  (set `/Game/Blueprints/GridLogic/BP_Grid.Occupied` true _asbp_grid)
  (`MaterialInstanceDynamic.SetVectorParameterValue` (`/Game/Blueprints/GridLogic/BP_Grid.GridMatRef` _asbp_grid) "None" (struct :`R` 0.084376 :`G` 0.887923 :`B` 1.0 :`A` 1.0)))

(event `ShowMovingGrids`
  (for _array_element (`self.RadiusToMove`)
    (`KismetArrayLibrary.Array_Add` (`self.RaduisToMoveResult`) (+ _array_element (`self.MyLocation`)))
    (bind _asbp_grid_setup (cast `/Game/Blueprints/GridLogic/BP_Grid_Setup` (`self.GetOwner`)))
    (for _array_element_2 (`/Game/Blueprints/GridLogic/BP_Grid_Setup.ArrayOfGrid` _asbp_grid_setup)
      (if (`KismetArrayLibrary.Array_Contains` (`self.RaduisToMoveResult`) (`/Game/Blueprints/GridLogic/BP_Grid.GridLocation` _array_element_2))
        (`KismetArrayLibrary.Array_Add` (`self.ArrayOfMovingGrid`) _array_element_2)))))

(event `ColoringGrids`
  (for _array_element (`self.ArrayOfMovingGrid`)
    (if (not (`/Game/Blueprints/GridLogic/BP_Grid.Occupied` _array_element))
      (set `/Game/Blueprints/GridLogic/BP_Grid.YouCanComeToMe` true _array_element)
      (`/Game/Blueprints/GridLogic/BP_Grid.AddTag` _array_element))))

(event `MoveToSelectedGrid`
  (params (SelectedGridLocation :type "Vector Structure"))
  (`AIBlueprintHelperLibrary.SimpleMoveToLocation` (`AIBlueprintHelperLibrary.GetAIController` null) SelectedGridLocation))

(fn `UserConstructionScript`
  (bind _returnvalue (`PrimitiveComponent.CreateDynamicMaterialInstance` (`self.Cone`) 0 "/Game/Materials/M_Unit.M_Unit" "None"))
  (set `self.GridMatRef` _returnvalue))