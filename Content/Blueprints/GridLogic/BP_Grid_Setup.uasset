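; Grid setup actor that builds the cell grid at BeginPlay and places a unit on it.
; Nested loops spawn GridX by GridY BP_Grid cells, spaced by GridSize around the actor's location, and store them in ArrayOfGrid.
; A five-second Delay inside the loop leads to SpawnUnit, which spawns a BP_Unit using separately randomized cell lookups for X and Y, with a hardcoded index range of 400.
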(event `self.ReceiveBeginPlay`
  (bind _gridx (`self.GridX`))
  (bind _gridy (`self.GridY`))
  (bind _gridsize (`self.GridSize`))
  (bind _gridsize_2 (`self.GridSize`))
  (for _index (range 1 (+ _gridx 1))
    (for _index_2 (range 1 (+ _gridy 1))
      (bind _returnvalue (`|SpawnActorFromClass` "/Game/Blueprints/GridLogic/BP_Grid.BP_Grid_C" (`KismetMathLibrary.MakeTransform` (+ (`KismetMathLibrary.MakeVector` (`KismetMathLibrary.Conv_IntToDouble` (- (* _index _gridsize_2) (/ (* _gridx _gridsize) 2))) (`KismetMathLibrary.Conv_IntToDouble` (- (* _index_2 _gridsize_2) (/ (* _gridy _gridsize) 2)))) (`self.K2_GetActorLocation`))) "AlwaysSpawn" "OverrideRootScale" self false null))
      ;[1 1 1] Добавление клеток в массив
      (`KismetArrayLibrary.Array_Add` (`self.ArrayOfGrid`) _returnvalue)
      (`KismetSystemLibrary.Delay` 5.0)
      (`self.SpawnUnit`))))

(event `SpawnUnit`
  (bind (_gridlocation_x _gridlocation_y) (`KismetMathLibrary.BreakVector` (`/Game/Blueprints/GridLogic/BP_Grid.GridLocation` (`|GetArrayItem` (`self.ArrayOfGrid`) (`KismetMathLibrary.RandomInteger` 400)))))
  (`|SpawnActorFromClass` "/Game/Blueprints/GameplayLogic/Units/BP_Unit.BP_Unit_C" (`KismetMathLibrary.MakeTransform` (`KismetMathLibrary.MakeVector` _gridlocation_x _gridlocation_y 10.0)) "AlwaysSpawn" "OverrideRootScale" self null))

(fn `UserConstructionScript`)