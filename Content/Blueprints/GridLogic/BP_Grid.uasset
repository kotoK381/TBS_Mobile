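; BP_Grid is a single grid tile that shows its world X and Y on a number widget and can highlight related tiles when clicked.
; Construction creates a dynamic material on its plane, and BeginPlay caches its location with Z zeroed.
; Click offsets that location by each Vector entry, then searches the owning BP_Grid_Setup's tile array and colors matches red.
; ChangeColor sets the tile's own color to black.
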(event `self.ReceiveBeginPlay`
  (bind (_returnvalue_x _returnvalue_y) (`KismetMathLibrary.BreakVector` (`self.K2_GetActorLocation`)))
  (bind _aswb_grid_number (cast `/Game/Blueprints/GridLogic/WB_GridNumber` (`WidgetComponent.GetUserWidgetObject` (`self.WB_Number`))))
  (`TextBlock.SetText` (`/Game/Blueprints/GridLogic/WB_GridNumber.NumberX` _aswb_grid_number) (`KismetTextLibrary.Conv_DoubleToText` _returnvalue_x "HalfToEven"))
  (`TextBlock.SetText` (`/Game/Blueprints/GridLogic/WB_GridNumber.NumberY` _aswb_grid_number) (`KismetTextLibrary.Conv_DoubleToText` _returnvalue_y "HalfToEven"))
  (set `self.GridLocation` (`KismetMathLibrary.MakeVector` _returnvalue_x _returnvalue_y)))

(event `ChangeColor`
  (`MaterialInstanceDynamic.SetVectorParameterValue` :`self` (`self.GridMatRef`) :`ParameterName` "Color"))

(event `Click`
  (for _array_element (`self.Vector`)
    (`KismetArrayLibrary.Array_Add` (`self.Vector_Result`) (+ _array_element (`self.GridLocation`)))
    (bind _asbp_grid_setup (cast `/Game/Blueprints/GridLogic/BP_Grid_Setup` (`self.GetOwner`)))
    (for _array_element_2 (`/Game/Blueprints/GridLogic/BP_Grid_Setup.ArrayOfGrid` _asbp_grid_setup)
      (if (`KismetArrayLibrary.Array_Contains` (`self.Vector_Result`) (`/Game/Blueprints/GridLogic/BP_Grid.GridLocation` _array_element_2))
        (`MaterialInstanceDynamic.SetVectorParameterValue` (`/Game/Blueprints/GridLogic/BP_Grid.GridMatRef` _array_element_2) "Color" (struct :`R` 1.0 :`B` 0.029524 :`A` 1.0))))))

(fn `UserConstructionScript`
  (bind _returnvalue (`PrimitiveComponent.CreateDynamicMaterialInstance` (`self.Plane`) 0 "/Game/Materials/M_grid.M_grid" "None"))
  (set `self.GridMatRef` _returnvalue))